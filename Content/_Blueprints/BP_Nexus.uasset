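; BP_Nexus links the game to an external device, apparently an IfMagic, over a wired COM-port stream and reads its orientation.
; BeginPlay opens the stream and, on success, starts a fast looping timer for polling; EndPlay disconnects.
; ReadStream converts the streamed dimension data to an orientation and prints its Euler rotation as debug output.
; The ForceUpdate event is an empty stub.
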(event Custom|ForceUpdate
  (params (Raw :type Integer) (Strength :type Integer)))

(event Custom|Read%20Stream
  (bind (_stream _returnvalue) (Class|Nexus|StreamDimension))
  (if _returnvalue
    (bind _eulerrot (Class|Nexus|Orientation _stream))
    (Development|PrintString (Utilities|String|ToString(Vector) _eulerrot))))

(event EventEndPlay
  (params (EndPlayReason :type EEndPlayReason%20Enum :default "Destroyed"))
  ;[1 1 1] Disconnected from the IfMagic
  (Class|Nexus|StreamDisconnect))

(event EventBeginPlay
  (bind _returnvalue (Class|Nexus|StreamConnect "7" false)) ; PC: Com 4 \\\ Laptop: COM 9
  (if _returnvalue
    (Utilities|Time|SetTimerbyEvent (EventDispatchers|CreateEvent :!event Custom|Read%20Stream) 0.1 true)))